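; BP_Nug_Emitter is a spawner actor that continuously emits BigNug actors from the world location of its Cube component.
; From BeginPlay it runs an endless loop, spawning a nug with a fixed speed and straight-down direction, then waiting a short random delay before repeating.
; A randomized positional offset from the Cube is present in the graph but left unconnected, so every nug spawns at the same point relative to it.
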(event `self.ReceiveBeginPlay`
  (`|SpawnActorFromClass` "/Game/B_P/BigNug.BigNug_C" (`KismetMathLibrary.Conv_VectorToTransform` (`SceneComponent.K2_GetComponentLocation` (`self.Cube`))) "Undefined" "OverrideRootScale" null 50.0 (0.0 0.0 -1.0) :!label _label)
  (`KismetSystemLibrary.Delay` (`KismetMathLibrary.RandomFloatInRange` 1.0 3.0))
  (goto _label))

(fn `UserConstructionScript`)